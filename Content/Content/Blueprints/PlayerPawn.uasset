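; Player pawn that handles vertical look, camera clipping and local HUD setup.
; Look-up input adds controller pitch and passes the clamped control-to-actor pitch delta to LookUpToServer, which stores it in LookUpAxis.
; Each tick it hides the mesh from its owner while the capsule overlaps CameraVisibilitySphere.
; On BeginPlay, only a locally controlled pawn creates the HUD, crosshair and health bar widgets.
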(event `LookUpToServer`
  (params (LookUpAxis :type "Float (double-precision)"))
  (set `self.LookUpAxis` LookUpAxis))

(event `InputAxis|LookUp`
  (params (AxisValue :type "Float (single-precision)"))
  (`self.LookUpToServer` (`KismetMathLibrary.ClampAngle` (.pitch (`KismetMathLibrary.NormalizedDeltaRotator` (`self.GetControlRotation`) (`self.K2_GetActorRotation`))) -90.0 90.0))
  (`self.AddControllerPitchInput` AxisValue))

(event `self.ReceiveTick`
  (params (DeltaSeconds :type "Float (single-precision)"))
  (bind _mesh (`self.Mesh`))
  (if (`PrimitiveComponent.IsOverlappingComponent` (`self.CapsuleComponent`) (`self.CameraVisibilitySphere`))
    (`PrimitiveComponent.SetOwnerNoSee` _mesh true)
    (else
      (`PrimitiveComponent.SetOwnerNoSee` _mesh false))))

(event `self.ReceiveBeginPlay`
  (if (`self.IsLocallyControlled`)
    (`|ExecutionSequence`
      (:`then_0`
        (bind _returnvalue (`|CreateWidget` "/Game/UI/WBP_HUD.WBP_HUD_C"))
        (`UserWidget.AddToViewport` _returnvalue 0))
      (:`then_1`
        (bind _returnvalue_2 (`|CreateWidget` "/Game/UI/WBP_Crosshair.WBP_Crosshair_C"))
        (`UserWidget.AddToViewport` _returnvalue_2 0))
      (:`then_2`
        (bind _returnvalue_3 (`|CreateWidget` "/Game/UI/WBP_HealthBar.WBP_HealthBar_C"))
        (`UserWidget.AddToViewport` _returnvalue_3 0)))))

(fn `UserConstructionScript`)
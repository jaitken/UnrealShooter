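; BP_ShotgunAI is a shotgun enemy pawn driven by the BT_ShotgunAI behavior tree, which its AI controller starts on BeginPlay.
; Tick stores the clamped pitch difference between control and actor rotation in LookUpAxis.
; A SpawnAmmo event rolls for a drop at the actor's location: a random power-up, otherwise possibly a shotgun or light ammo pickup, or nothing.
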(event `self.ReceiveTick`
  (params (DeltaSeconds :type "Float (single-precision)"))
  (set `self.LookUpAxis` (`KismetMathLibrary.ClampAngle` (.pitch (`KismetMathLibrary.NormalizedDeltaRotator` (`self.GetControlRotation`) (`self.K2_GetActorRotation`))) -90.0 90.0)))

(event `self.ReceiveBeginPlay`
  (bind _returnvalue (`AIBlueprintHelperLibrary.GetAIController` self))
  (`/Engine/EditorBlueprintResources/StandardMacros.IsValid` _returnvalue
    (:`Is Valid`
      (`AIController.RunBehaviorTree` _returnvalue "/Game/Enemies/ShotgunAI/BT_ShotgunAI.BT_ShotgunAI"))))

(event `self.SpawnAmmo`
  (bind _returnvalue (`self.K2_GetActorLocation` self))
  (if (< (`KismetMathLibrary.RandomInteger` 100) 30)
    (`|SpawnActorFromClass` (select `int` (`KismetMathLibrary.RandomInteger` 3) :`0` "/Game/Powerups/TestSuperSpeed.TestSuperSpeed_C" :`1` "/Game/Powerups/TestQuadDamage.TestQuadDamage_C" :`2` "/Game/Powerups/TestHealthRegen.TestHealthRegen_C" :!type "Actor Class Reference") (`KismetMathLibrary.Conv_VectorToTransform` _returnvalue) "AdjustIfPossibleButAlwaysSpawn" "OverrideRootScale" null null)
    (elif (< (`KismetMathLibrary.RandomInteger` 100) 40)
      (`|SpawnActorFromClass` (select `int` (`KismetMathLibrary.RandomInteger` 2) :`0` "/Game/Blueprints/BP_ShotgunAmmoPickup.BP_ShotgunAmmoPickup_C" :`1` "/Game/Blueprints/BP_LightAmmoPickup.BP_LightAmmoPickup_C" :!type "Actor Class Reference") (`KismetMathLibrary.Conv_VectorToTransform` _returnvalue) "AdjustIfPossibleButAlwaysSpawn" "OverrideRootScale" null null))))

(fn `UserConstructionScript`)
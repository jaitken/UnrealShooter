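; BP_Door is a door actor that shows a text label when the player comes near; it contains no open or close logic.
; The construction script copies the DoorText variable into two text render components.
; Each Tick, it checks the player pawn's distance, shows both texts within a fixed range and hides them beyond it.
; While visible, both texts rotate toward the player camera using a look-at rotation from the actor's origin.
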(event `self.ReceiveTick`
  (params (DeltaSeconds :type "Float (single-precision)"))
  (bind _returnvalue (`GameplayStatics.GetPlayerPawn` 0))
  (bind _textrender (`self.TextRender`))
  (bind _textrender1 (`self.TextRender1`))
  (bind _returnvalue_2 (`KismetMathLibrary.FindLookAtRotation` (`self.K2_GetActorLocation`) (`self.K2_GetActorLocation` (`PlayerController.PlayerCameraManager` (`GameplayStatics.GetPlayerController` 0)))))
  (`/Engine/EditorBlueprintResources/StandardMacros.IsValid` _returnvalue
    (:`Is Valid`
      (if (< (`KismetMathLibrary.VSize` (- (`self.K2_GetActorLocation` _returnvalue) (`self.K2_GetActorLocation`))) 600.0)
        (`SceneComponent.SetVisibility` _textrender1 true false)
        (`SceneComponent.SetVisibility` _textrender true false)
        (`SceneComponent.K2_SetWorldRotation` (`self.TextRender`) _returnvalue_2 false false)
        (`SceneComponent.K2_SetWorldRotation` (`self.TextRender1`) _returnvalue_2 false false)
        (else
          (`SceneComponent.SetVisibility` _textrender1 false false)
          (`SceneComponent.SetVisibility` _textrender false false))))))

(fn `UserConstructionScript`
  (`TextRenderComponent.K2_SetText` (`self.TextRender`) (`self.DoorText`))
  (`TextRenderComponent.K2_SetText` (`self.TextRender1`) (`self.DoorText`)))
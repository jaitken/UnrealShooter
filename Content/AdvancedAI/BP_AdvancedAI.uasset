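; BP_AdvancedAI is an AI-controlled character that runs BT_AdvancedAI through its AI controller on BeginPlay.
; Each tick it stores the control-to-actor pitch difference in LookUpAxis, clamped to straight down and straight up.
; A SpawnAmmo event, with no caller in this graph, gives a one-in-four chance of spawning an AR ammo pickup at its location.
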(event `self.ReceiveTick`
  (params (DeltaSeconds :type "Float (single-precision)"))
  (set `self.LookUpAxis` (`KismetMathLibrary.ClampAngle` (.pitch (`KismetMathLibrary.NormalizedDeltaRotator` (`self.GetControlRotation`) (`self.K2_GetActorRotation`))) -90.0 90.0)))

(event `self.ReceiveBeginPlay`
  (bind _returnvalue (`AIBlueprintHelperLibrary.GetAIController` self))
  (`/Engine/EditorBlueprintResources/StandardMacros.IsValid` _returnvalue
    (:`Is Valid`
      (`AIController.RunBehaviorTree` _returnvalue "/Game/AdvancedAI/BT_AdvancedAI.BT_AdvancedAI"))))

(event `self.SpawnAmmo`
  (if (< (`KismetMathLibrary.RandomInteger` 100) 25)
    (`|SpawnActorFromClass` "/Game/Blueprints/BP_ARAmmoPickup.BP_ARAmmoPickup_C" (`KismetMathLibrary.Conv_VectorToTransform` (`self.K2_GetActorLocation` self)) "Undefined" "OverrideRootScale" null null)))

(fn `UserConstructionScript`)
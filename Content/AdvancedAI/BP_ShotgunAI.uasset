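; BP_ShotgunAI is an AI-controlled pawn Blueprint for a shotgun enemy or NPC, driven by a behavior tree.
; On BeginPlay it runs BT_ShotgunAI through its AI controller, if that controller is valid.
; Each Tick it stores the pitch difference between control and actor rotation, clamped to straight down and straight up, in LookUpAxis.
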(event `self.ReceiveTick`
  (params (DeltaSeconds :type "Float (single-precision)"))
  (set `self.LookUpAxis` (`KismetMathLibrary.ClampAngle` (.pitch (`KismetMathLibrary.NormalizedDeltaRotator` (`self.GetControlRotation`) (`self.K2_GetActorRotation`))) -90.0 90.0)))

(event `self.ReceiveBeginPlay`
  (bind _returnvalue (`AIBlueprintHelperLibrary.GetAIController` self))
  (`/Engine/EditorBlueprintResources/StandardMacros.IsValid` _returnvalue
    (:`Is Valid`
      (`AIController.RunBehaviorTree` _returnvalue "/Game/AdvancedAI/BT_ShotgunAI.BT_ShotgunAI"))))

(fn `UserConstructionScript`)
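; Double-barrel weapon pickup actor that shows a floating text label when the player is nearby; the graphs here contain no pickup logic.
; The construction script fills the TextRender from the TextAbove variable.
; Each Tick checks the distance to player pawn 0, shows the label within a short radius, and rotates it toward the player camera.
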(event `self.ReceiveTick`
  (params (DeltaSeconds :type "Float (single-precision)"))
  (bind _returnvalue (`GameplayStatics.GetPlayerPawn` 0))
  (bind _textrender (`self.TextRender`))
  (`/Engine/EditorBlueprintResources/StandardMacros.IsValid` _returnvalue
    (:`Is Valid`
      (if (< (`KismetMathLibrary.VSize` (- (`self.K2_GetActorLocation` _returnvalue) (`self.K2_GetActorLocation`))) 300.0)
        (`SceneComponent.SetVisibility` _textrender true false)
        (`SceneComponent.K2_SetWorldRotation` (`self.TextRender`) (`KismetMathLibrary.FindLookAtRotation` (`self.K2_GetActorLocation`) (`self.K2_GetActorLocation` (`PlayerController.PlayerCameraManager` (`GameplayStatics.GetPlayerController` 0)))) false false)
        (else
          (`SceneComponent.SetVisibility` _textrender false false))))))

(fn `UserConstructionScript`
  (`TextRenderComponent.K2_SetText` (`self.TextRender`) (`self.TextAbove`)))